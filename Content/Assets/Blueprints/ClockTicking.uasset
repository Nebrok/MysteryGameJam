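; Clock Blueprint that advances a second hand and announces when a minute has run out.
; While ticking is allowed, Tick accumulates delta time and, each time it passes one second, rolls the hand by six degrees per elapsed second.
; It then clears the accumulator and increments a seconds counter, printing a time-up message when that counter hits sixty.
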(event `self.ReceiveTick`
  (params (DeltaSeconds :type "Float (single-precision)"))
  (bind _secondhand (`self.SecondHand`))
  (if (`self.AllowedToTick`)
    (bind _output_get (set `self.TimeElapsed` (+ (`self.TimeElapsed`) DeltaSeconds)))
    (`/Engine/EditorBlueprintResources/StandardMacros.CompareFloat` _output_get 1.0
      (:`>`
        (`SceneComponent.K2_SetRelativeRotation` _secondhand (`KismetMathLibrary.ComposeRotators` (`SceneComponent.RelativeRotation` _secondhand) (`KismetMathLibrary.MakeRotator` (* _output_get 6.0))) false false)
        (`|ExecutionSequence`
          (:`then_0`
            (set `self.TimeElapsed` 0.0))
          (:`then_1`
            (bind _result (`/Engine/EditorBlueprintResources/StandardMacros.IncrementInt` (`self.Seconds Elapsed`))
              (:`  `
                (`/Engine/EditorBlueprintResources/StandardMacros.CompareInt` _result 60
                  (:`==`
                    (`KismetSystemLibrary.PrintString` "Time is up")))))))))))