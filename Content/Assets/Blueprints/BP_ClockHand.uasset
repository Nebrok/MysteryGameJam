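; BP_ClockHand is an actor that steps a Cube around like the second hand of a clock.
; While AllowedToTick is set, Tick accumulates delta time and, once it passes one second, rolls the Cube six degrees per elapsed second.
; It then zeroes the timer, discarding any overshoot, and increments and prints SecondsElapsed.
; A final comparison against 60 has nothing wired to its outputs.
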(event `self.ReceiveTick`
  (params (DeltaSeconds :type "Float (single-precision)"))
  (bind _cube (`self.Cube`))
  (if (`self.AllowedToTick`)
    (bind _output_get (set `self.TimeElapsed` (+ (`self.TimeElapsed`) DeltaSeconds)))
    (`/Engine/EditorBlueprintResources/StandardMacros.CompareFloat` _output_get 1.0
      (:`>`
        (`SceneComponent.K2_SetRelativeRotation` _cube (`KismetMathLibrary.ComposeRotators` (`SceneComponent.RelativeRotation` _cube) (`KismetMathLibrary.MakeRotator` (* _output_get 6.0))) false false)
        (`|ExecutionSequence`
          (:`then_0`
            (set `self.TimeElapsed` 0.0))
          (:`then_1`
            (bind _result (`/Engine/EditorBlueprintResources/StandardMacros.IncrementInt` (`self.SecondsElapsed`))
              (:`  `
                (`KismetSystemLibrary.PrintString` (`KismetStringLibrary.Conv_IntToString` _result))
                (`/Engine/EditorBlueprintResources/StandardMacros.CompareInt` _result 60)))))))))

(fn `UserConstructionScript`)